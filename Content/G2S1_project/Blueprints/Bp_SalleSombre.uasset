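; Dark-room actor that shows a screen overlay depending on which actor overlaps it.
; The cat, detected by comparing the instance name to "Bp_chat_C_0", gets the Nyctalopie (night vision) widget, while any other actor gets FullSombre (full darkness).
; Each widget is created on its first matching overlap, then made visible again on later ones.
; Any end overlap collapses both widgets.
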(event `self.ReceiveActorBeginOverlap`
  (params (OtherActor :type "Actor Object Reference"))
  (if (`KismetStringLibrary.NotEqual_StrStr` (`KismetStringLibrary.Conv_ObjectToString` OtherActor) "Bp_chat_C_0")
    (if (`self.1er passageAutre`)
      (`Widget.SetVisibility` (`self.wid_fullsombre`) "Visible")
      (else
        (set `self.1er passageAutre` true)
        (bind _returnvalue (`|CreateWidget` "/Game/G2S1_project/Widgets/FullSombre.FullSombre_C"))
        (set `self.wid_fullsombre` _returnvalue)
        (`UserWidget.AddToViewport` _returnvalue 0)))
    (elif (`self.1er passageCatty`)
      (`Widget.SetVisibility` (`self.wid_nyctalopie`) "Visible")
      (else
        (set `self.1er passageCatty` true)
        (bind _returnvalue_2 (`|CreateWidget` "/Game/G2S1_project/Widgets/nyctalopie.nyctalopie_C"))
        (set `self.wid_nyctalopie` _returnvalue_2)
        (`UserWidget.AddToViewport` _returnvalue_2 0)))))

(event `self.ReceiveActorEndOverlap`
  (params (OtherActor :type "Actor Object Reference"))
  (`Widget.SetVisibility` (`self.wid_nyctalopie`) "Collapsed")
  (`Widget.SetVisibility` (`self.wid_fullsombre`) "Collapsed"))

(fn `UserConstructionScript`)