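; Player cat character for a local two-player setup with a gorilla partner, handling movement input for both.
; BeginPlay creates a second player and caches the gorilla; Space makes that player's controller possess it.
; Picking up the GameBoy flags both characters, letting C toggle tagged RealWorld and OtherWorld actors' visibility and collision.
; Passage events briefly zero walk speed and launch the cat along an axis; gorilla-follow draft logic remains disconnected.
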(event `InputAxis|Turn Right / Left Mouse Gorille`
  (params (AxisValue :type "Float (single-precision)"))
  (`self.AddControllerYawInput` (`self.Gorille`) AxisValue))

(event `InputAxis|Move Forward / Backward Gorille`
  (params (AxisValue :type "Float (single-precision)"))
  (bind (_returnvalue_roll _returnvalue_pitch _returnvalue_yaw) (`KismetMathLibrary.BreakRotator` (`self.GetControlRotation` (`self.Gorille`))))
  (`self.AddMovementInput` (`self.Gorille`) (`KismetMathLibrary.GetForwardVector` (`KismetMathLibrary.MakeRotator` 0.0 0.0 _returnvalue_yaw)) AxisValue false))

(event `InputAxis|Move Right / Left Gorille`
  (params (AxisValue :type "Float (single-precision)"))
  (bind (_returnvalue_roll _returnvalue_pitch _returnvalue_yaw) (`KismetMathLibrary.BreakRotator` (`self.GetControlRotation` (`self.Gorille`))))
  (`self.AddMovementInput` (`self.Gorille`) (`KismetMathLibrary.GetRightVector` (`KismetMathLibrary.MakeRotator` _returnvalue_roll 0.0 _returnvalue_yaw)) AxisValue false))

(event `self.ReceiveBeginPlay`
  ;[1 1 1] Passage au gorille pour J2
  (if (<= (`GameplayStatics.GetNumPlayerControllers`) 1)
    (bind _returnvalue (`GameplayStatics.CreatePlayer` -1))
    (`self.SpawnDefaultController`)
    (set `self.Player 2` _returnvalue)
    (`KismetSystemLibrary.Delay` 0.5)
    (bind _returnvalue_2 (`GameplayStatics.GetActorOfClass` "/Game/G2S1_project/Blueprints/Bp_gorille.Bp_gorille_C"))
    (set `self.Gorille` _returnvalue_2)))

(event `Key|C`
  (params (Key :type "Key Structure"))
  ;[1 1 1] Changement de monde
  (:`Pressed`
    (if (`self.GameBoy`)
      (`KismetSystemLibrary.PrintString` "True C")
      (`/Engine/EditorBlueprintResources/StandardMacros.FlipFlop`
        (:`A`
          (bind _outactors (`GameplayStatics.GetAllActorsWithTag` "RealWorld"))
          (`self.SetActorEnableCollision` _outactors false)
          (`self.SetActorHiddenInGame` _outactors true)
          (bind _outactors_2 (`GameplayStatics.GetAllActorsWithTag` "OtherWorld"))
          (`self.SetActorEnableCollision` _outactors_2 true)
          (`self.SetActorHiddenInGame` _outactors_2 false))
        (:`B`
          (bind _outactors_3 (`GameplayStatics.GetAllActorsWithTag` "RealWorld"))
          (`self.SetActorEnableCollision` _outactors_3 true)
          (`self.SetActorHiddenInGame` _outactors_3 false)
          (bind _outactors_4 (`GameplayStatics.GetAllActorsWithTag` "OtherWorld"))
          (`self.SetActorEnableCollision` _outactors_4 false)
          (`self.SetActorHiddenInGame` _outactors_4 true))))))

(event `ChoppeGameBoy`
  ;[1 1 1] Changement de monde
  (set `self.GameBoy` true)
  (bind _asbp_gorille (cast `/Game/G2S1_project/Blueprints/Bp_gorille` (`self.Gorille`)))
  (set `/Game/G2S1_project/Blueprints/Bp_gorille.GameBoy` true _asbp_gorille))

(event `InputAxis|Turn Right / Left Mouse Cat`
  (params (AxisValue :type "Float (single-precision)"))
  ;[1 1 1] Déplacement
  (set `self.YawAxis` AxisValue)
  (`self.AddControllerYawInput` AxisValue))

(event `Gorille Forward`
  (bind (_returnvalue_roll _returnvalue_pitch _returnvalue_yaw) (`KismetMathLibrary.BreakRotator` (`self.GetControlRotation`)))
  ;[1 1 1] Brouillon Gorille follow 1 joueur
  (`Timeline|Timeline_0`
    (:`Finished`
      (`self.AddMovementInput` (`self.Gorille`) (`KismetMathLibrary.GetForwardVector` (`KismetMathLibrary.MakeRotator` 0.0 0.0 _returnvalue_yaw)) (`self.ForwardAxis`) false))))

(event `InputAxis|Move Forward / Backward Cat`
  (params (AxisValue :type "Float (single-precision)"))
  (bind (_returnvalue_roll _returnvalue_pitch _returnvalue_yaw) (`KismetMathLibrary.BreakRotator` (`self.GetControlRotation`)))
  ;[1 1 1] Déplacement
  (set `self.ForwardAxis` AxisValue)
  (`self.AddMovementInput` (`KismetMathLibrary.GetForwardVector` (`KismetMathLibrary.MakeRotator` 0.0 0.0 _returnvalue_yaw)) AxisValue))

(event `InputAxis|Move Right / Left Cat`
  (params (AxisValue :type "Float (single-precision)"))
  (bind (_returnvalue_roll _returnvalue_pitch _returnvalue_yaw) (`KismetMathLibrary.BreakRotator` (`self.GetControlRotation`)))
  ;[1 1 1] Déplacement
  (set `self.LateralAxis` AxisValue)
  (`self.AddMovementInput` (`KismetMathLibrary.GetRightVector` (`KismetMathLibrary.MakeRotator` _returnvalue_roll 0.0 _returnvalue_yaw)) AxisValue))

(event `Gorille Lateral`
  (bind (_returnvalue_roll _returnvalue_pitch _returnvalue_yaw) (`KismetMathLibrary.BreakRotator` (`self.GetControlRotation`)))
  ;[1 1 1] Brouillon Gorille follow 1 joueur
  (`self.AddMovementInput` (`self.Gorille`) (`KismetMathLibrary.GetRightVector` (`KismetMathLibrary.MakeRotator` _returnvalue_roll 0.0 _returnvalue_yaw)) (`self.LateralAxis`) false))

(event `Key|SpaceBar`
  (params (Key :type "Key Structure"))
  ;[1 1 1] Changement perso
  (:`Pressed`
    (`self.Switch au gorille`)))

(event `Switch au gorille`
  ;[1 1 1] Changement perso
  (bind _returnvalue (`GameplayStatics.GetActorOfClass` "/Game/G2S1_project/Blueprints/Bp_gorille.Bp_gorille_C"))
  (`Controller.Possess` (`GameplayStatics.GetPlayerController` 1) _returnvalue))

(event `PassageDroiteGauche`
  ;[1 1 1] Passages étroit
  (set `CharacterMovementComponent.MaxWalkSpeed` 0.0 (`self.CharacterMovement`))
  (`MovementComponent.StopMovementImmediately` (`self.CharacterMovement`))
  (`self.LaunchCharacter` (-2000.0 0.0 0.0))
  (`KismetSystemLibrary.Delay` 0.2)
  (set `CharacterMovementComponent.MaxWalkSpeed` 600.0 (`self.CharacterMovement`)))

(event `PassageGaucheDroite`
  ;[1 1 1] Passages étroit
  (set `CharacterMovementComponent.MaxWalkSpeed` 0.0 (`self.CharacterMovement`))
  (`MovementComponent.StopMovementImmediately` (`self.CharacterMovement`))
  (`self.LaunchCharacter` (2000.0 0.0 0.0))
  (`KismetSystemLibrary.Delay` 0.2)
  (set `CharacterMovementComponent.MaxWalkSpeed` 600.0 (`self.CharacterMovement`)))

(event `PassageHautBas`
  ;[1 1 1] Passages étroit
  (set `CharacterMovementComponent.MaxWalkSpeed` 0.0 (`self.CharacterMovement`))
  (`MovementComponent.StopMovementImmediately` (`self.CharacterMovement`))
  (`self.LaunchCharacter` (0.0 2000.0 0.0))
  (`KismetSystemLibrary.Delay` 0.2)
  (set `CharacterMovementComponent.MaxWalkSpeed` 600.0 (`self.CharacterMovement`)))

(event `PassageBasHaut`
  ;[1 1 1] Passages étroit
  (set `CharacterMovementComponent.MaxWalkSpeed` 0.0 (`self.CharacterMovement`))
  (`MovementComponent.StopMovementImmediately` (`self.CharacterMovement`))
  (`self.LaunchCharacter` (0.0 -2000.0 0.0))
  (`KismetSystemLibrary.Delay` 0.2)
  (set `CharacterMovementComponent.MaxWalkSpeed` 600.0 (`self.CharacterMovement`)))

(event `Key|BackSpace`
  (params (Key :type "Key Structure"))
  (:`Pressed`
    (`KismetSystemLibrary.PrintString` "Destruction attempt")
    (`GameplayStatics.RemovePlayer` (`GameplayStatics.GetPlayerControllerFromID` 2) true)))

(fn `UserConstructionScript`)