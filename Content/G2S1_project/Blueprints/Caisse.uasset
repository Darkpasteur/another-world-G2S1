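; Crate actor that the gorilla character can grab and release through the KongInteract event.
; Four side collisions (right, left, top, bottom) find which side the gorilla overlaps, turning it to a matching fixed yaw and stopping its movement.
; After a brief delay the crate attaches to the gorilla, keeping world transform; interacting again detaches it.
; The held state lives in GorilleRestrained on Bp_chat, the cat, rather than on the crate.
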(event `Kong Interact`
  (bind _returnvalue (`GameplayStatics.GetActorOfClass` "/Game/G2S1_project/Blueprints/Bp_gorille.Bp_gorille_C"))
  (set `self.Gorilla` _returnvalue)
  (bind _returnvalue_2 (`GameplayStatics.GetActorOfClass` "/Game/G2S1_project/Blueprints/Bp_chat.Bp_chat_C"))
  (set `self.Catty` _returnvalue_2)
  (if (`PrimitiveComponent.IsOverlappingActor` (`self.Collision droite`) (`self.Gorilla`))
    (bind _asbp_chat (cast `/Game/G2S1_project/Blueprints/Bp_chat` (`self.Catty`)))
    (if (`/Game/G2S1_project/Blueprints/Bp_chat.Gorille restrained` _asbp_chat)
      (`self.K2_DetachFromActor` "KeepWorld" "KeepWorld" "KeepWorld")
      (bind _asbp_chat_2 (cast `/Game/G2S1_project/Blueprints/Bp_chat` (`self.Catty`)))
      (set `/Game/G2S1_project/Blueprints/Bp_chat.Gorille restrained` false _asbp_chat_2)
      (cast `/Game/G2S1_project/Blueprints/Bp_gorille` (`self.Gorilla`))
      (else
        (`Controller.SetControlRotation` (`Pawn.GetController` (`self.Gorilla`)) (`KismetMathLibrary.MakeRotator` 0.0 0.0 180.0))
        (`MovementComponent.StopMovementImmediately` (`Character.CharacterMovement` (`self.Gorilla`)))
        (`KismetSystemLibrary.Delay` 0.05)
        (`self.K2_AttachToActor` (`self.Gorilla`) "None" "KeepWorld" "KeepWorld" "KeepWorld" false)
        (bind _asbp_chat_3 (cast `/Game/G2S1_project/Blueprints/Bp_chat` (`self.Catty`)))
        (set `/Game/G2S1_project/Blueprints/Bp_chat.Gorille restrained` true _asbp_chat_3)
        (cast `/Game/G2S1_project/Blueprints/Bp_gorille` (`self.Gorilla`))))
    (elif (`PrimitiveComponent.IsOverlappingActor` (`self.Collision gauche`) (`self.Gorilla`))
      (bind _asbp_chat_4 (cast `/Game/G2S1_project/Blueprints/Bp_chat` (`self.Catty`)))
      (if (`/Game/G2S1_project/Blueprints/Bp_chat.Gorille restrained` _asbp_chat_4)
        (`self.K2_DetachFromActor` "KeepWorld" "KeepWorld" "KeepWorld")
        (bind _asbp_chat_5 (cast `/Game/G2S1_project/Blueprints/Bp_chat` (`self.Catty`)))
        (set `/Game/G2S1_project/Blueprints/Bp_chat.Gorille restrained` false _asbp_chat_5)
        (cast `/Game/G2S1_project/Blueprints/Bp_gorille` (`self.Gorilla`))
        (else
          (`Controller.SetControlRotation` (`Pawn.GetController` (`self.Gorilla`)) (`KismetMathLibrary.MakeRotator` 0.0 0.0 0.0))
          (`MovementComponent.StopMovementImmediately` (`Character.CharacterMovement` (`self.Gorilla`)))
          (`KismetSystemLibrary.Delay` 0.05)
          (`self.K2_AttachToActor` (`self.Gorilla`) "None" "KeepWorld" "KeepWorld" "KeepWorld" false)
          (bind _asbp_chat_6 (cast `/Game/G2S1_project/Blueprints/Bp_chat` (`self.Catty`)))
          (set `/Game/G2S1_project/Blueprints/Bp_chat.Gorille restrained` true _asbp_chat_6)
          (cast `/Game/G2S1_project/Blueprints/Bp_gorille` (`self.Gorilla`))))
      (elif (`PrimitiveComponent.IsOverlappingActor` (`self.Collision haut `) (`self.Gorilla`))
        (bind _asbp_chat_7 (cast `/Game/G2S1_project/Blueprints/Bp_chat` (`self.Catty`)))
        (if (`/Game/G2S1_project/Blueprints/Bp_chat.Gorille restrained` _asbp_chat_7)
          (`self.K2_DetachFromActor` "KeepWorld" "KeepWorld" "KeepWorld")
          (bind _asbp_chat_8 (cast `/Game/G2S1_project/Blueprints/Bp_chat` (`self.Catty`)))
          (set `/Game/G2S1_project/Blueprints/Bp_chat.Gorille restrained` false _asbp_chat_8)
          (else
            (`Controller.SetControlRotation` (`Pawn.GetController` (`self.Gorilla`)) (`KismetMathLibrary.MakeRotator` 0.0 0.0 90.0))
            (`MovementComponent.StopMovementImmediately` (`Character.CharacterMovement` (`self.Gorilla`)))
            (`KismetSystemLibrary.Delay` 0.05)
            (`self.K2_AttachToActor` (`self.Gorilla`) "None" "KeepWorld" "KeepWorld" "KeepWorld" false)
            (bind _asbp_chat_9 (cast `/Game/G2S1_project/Blueprints/Bp_chat` (`self.Catty`)))
            (set `/Game/G2S1_project/Blueprints/Bp_chat.Gorille restrained` true _asbp_chat_9)))
        (elif (`PrimitiveComponent.IsOverlappingActor` (`self.Collision bas`) (`self.Gorilla`))
          (bind _asbp_chat_10 (cast `/Game/G2S1_project/Blueprints/Bp_chat` (`self.Catty`)))
          (if (`/Game/G2S1_project/Blueprints/Bp_chat.Gorille restrained` _asbp_chat_10)
            (`self.K2_DetachFromActor` "KeepWorld" "KeepWorld" "KeepWorld")
            (bind _asbp_chat_11 (cast `/Game/G2S1_project/Blueprints/Bp_chat` (`self.Catty`)))
            (set `/Game/G2S1_project/Blueprints/Bp_chat.Gorille restrained` false _asbp_chat_11)
            (else
              (`Controller.SetControlRotation` (`Pawn.GetController` (`self.Gorilla`)) (`KismetMathLibrary.MakeRotator` 0.0 0.0 270.0))
              (`MovementComponent.StopMovementImmediately` (`Character.CharacterMovement` (`self.Gorilla`)))
              (`KismetSystemLibrary.Delay` 0.05)
              (`self.K2_AttachToActor` (`self.Gorilla`) "None" "KeepWorld" "KeepWorld" "KeepWorld" false)
              (bind _asbp_chat_12 (cast `/Game/G2S1_project/Blueprints/Bp_chat` (`self.Catty`)))
              (set `/Game/G2S1_project/Blueprints/Bp_chat.Gorille restrained` true _asbp_chat_12))))))))

(fn `UserConstructionScript`)