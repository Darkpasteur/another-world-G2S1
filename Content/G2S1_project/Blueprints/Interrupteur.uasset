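; Light switch actor that lights dark rooms (Bp_SalleSombre) whose NuméroSalle matches its NuméroInterrupteur.
; The Lumière event, while Bp_chat overlaps the switch, sets Allumé, hides each matching room's Obscurité and disables its five collision components.
; The cat leaving while Allumé is set restores darkness and collision and clears the flag.
; The lacherinterrupteur release event also restores them during overlap, but leaves Allumé true.
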(event `Lumière`
  (bind _returnvalue (`GameplayStatics.GetActorOfClass` "/Game/G2S1_project/Blueprints/Bp_chat.Bp_chat_C"))
  (if (`self.IsOverlappingActor` _returnvalue)
    (set `self.allumé` true)
    (bind _outactors (`GameplayStatics.GetAllActorsOfClass` "/Game/G2S1_project/Blueprints/Bp_SalleSombre.Bp_SalleSombre_C"))
    (for _array_element _outactors
      (if (== (`/Game/G2S1_project/Blueprints/Bp_SalleSombre.Numéro Salle` _array_element) (`self.Numéro interrupteur`))
        (`SceneComponent.SetVisibility` (`/Game/G2S1_project/Blueprints/Bp_SalleSombre.Obscurité` _array_element) false false)
        (`PrimitiveComponent.SetCollisionEnabled` (`/Game/G2S1_project/Blueprints/Bp_SalleSombre.Collision` _array_element) "NoCollision")
        (`PrimitiveComponent.SetCollisionEnabled` (`/Game/G2S1_project/Blueprints/Bp_SalleSombre.CollisionEst` _array_element) "NoCollision")
        (`PrimitiveComponent.SetCollisionEnabled` (`/Game/G2S1_project/Blueprints/Bp_SalleSombre.CollisionSud` _array_element) "NoCollision")
        (`PrimitiveComponent.SetCollisionEnabled` (`/Game/G2S1_project/Blueprints/Bp_SalleSombre.CollisionNord` _array_element) "NoCollision")
        (`PrimitiveComponent.SetCollisionEnabled` (`/Game/G2S1_project/Blueprints/Bp_SalleSombre.CollisionOuest` _array_element) "NoCollision")))))

(event `self.ReceiveActorEndOverlap`
  (params (OtherActor :type "Actor Object Reference"))
  (bind _returnvalue (`GameplayStatics.GetActorOfClass` "/Game/G2S1_project/Blueprints/Bp_chat.Bp_chat_C"))
  (if (== _returnvalue OtherActor)
    (if (`self.allumé`)
      (set `self.allumé` false)
      (bind _outactors (`GameplayStatics.GetAllActorsOfClass` "/Game/G2S1_project/Blueprints/Bp_SalleSombre.Bp_SalleSombre_C"))
      (for _array_element _outactors
        (if (== (`/Game/G2S1_project/Blueprints/Bp_SalleSombre.Numéro Salle` _array_element) (`self.Numéro interrupteur`))
          (`SceneComponent.SetVisibility` (`/Game/G2S1_project/Blueprints/Bp_SalleSombre.Obscurité` _array_element) true false)
          (`PrimitiveComponent.SetCollisionEnabled` (`/Game/G2S1_project/Blueprints/Bp_SalleSombre.Collision` _array_element) "QueryAndPhysics")
          (`PrimitiveComponent.SetCollisionEnabled` (`/Game/G2S1_project/Blueprints/Bp_SalleSombre.CollisionEst` _array_element) "QueryAndPhysics")
          (`PrimitiveComponent.SetCollisionEnabled` (`/Game/G2S1_project/Blueprints/Bp_SalleSombre.CollisionSud` _array_element) "QueryAndPhysics")
          (`PrimitiveComponent.SetCollisionEnabled` (`/Game/G2S1_project/Blueprints/Bp_SalleSombre.CollisionNord` _array_element) "QueryAndPhysics")
          (`PrimitiveComponent.SetCollisionEnabled` (`/Game/G2S1_project/Blueprints/Bp_SalleSombre.CollisionOuest` _array_element) "QueryAndPhysics"))))))

(event `lacher interrupteur`
  (bind _returnvalue (`GameplayStatics.GetActorOfClass` "/Game/G2S1_project/Blueprints/Bp_chat.Bp_chat_C"))
  (if (`self.IsOverlappingActor` _returnvalue)
    (set `self.allumé` true)
    (bind _outactors (`GameplayStatics.GetAllActorsOfClass` "/Game/G2S1_project/Blueprints/Bp_SalleSombre.Bp_SalleSombre_C"))
    (for _array_element _outactors
      (if (== (`/Game/G2S1_project/Blueprints/Bp_SalleSombre.Numéro Salle` _array_element) (`self.Numéro interrupteur`))
        (`SceneComponent.SetVisibility` (`/Game/G2S1_project/Blueprints/Bp_SalleSombre.Obscurité` _array_element) true false)
        (`PrimitiveComponent.SetCollisionEnabled` (`/Game/G2S1_project/Blueprints/Bp_SalleSombre.Collision` _array_element) "QueryAndPhysics")
        (`PrimitiveComponent.SetCollisionEnabled` (`/Game/G2S1_project/Blueprints/Bp_SalleSombre.CollisionEst` _array_element) "QueryAndPhysics")
        (`PrimitiveComponent.SetCollisionEnabled` (`/Game/G2S1_project/Blueprints/Bp_SalleSombre.CollisionSud` _array_element) "QueryAndPhysics")
        (`PrimitiveComponent.SetCollisionEnabled` (`/Game/G2S1_project/Blueprints/Bp_SalleSombre.CollisionNord` _array_element) "QueryAndPhysics")
        (`PrimitiveComponent.SetCollisionEnabled` (`/Game/G2S1_project/Blueprints/Bp_SalleSombre.CollisionOuest` _array_element) "QueryAndPhysics")))))

(fn `UserConstructionScript`)