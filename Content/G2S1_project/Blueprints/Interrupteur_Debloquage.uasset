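; Light switch actor that unlocks dark rooms (Bp_SalleSombre) whose room number matches its own, while Bp_chat holds it.
; A box overlap toggles a widget's visibility.
; With the cat overlapping, Lumière calls its ControlArthur, hides matching rooms' darkness and disables their collisions.
; The cat leaving while lit, or lacherinterrupteur while overlapping, restores darkness and collision, though the latter sets Allumé true.
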(event `self.Box.OnComponentBeginOverlap`
  (params (OverlappedComponent :type "PrimitiveComponent Object Reference") (OtherActor :type "Actor Object Reference") (OtherComp :type "PrimitiveComponent Object Reference") (OtherBodyIndex :type Integer) (bFromSweep :type Boolean) (SweepResult :type "HitResult Structure (by ref)"))
  (`SceneComponent.SetVisibility` (`self.Widget`) true false))

(event `self.Box.OnComponentEndOverlap`
  (params (OverlappedComponent :type "PrimitiveComponent Object Reference") (OtherActor :type "Actor Object Reference") (OtherComp :type "PrimitiveComponent Object Reference") (OtherBodyIndex :type Integer))
  (`SceneComponent.SetVisibility` (`self.Widget`) false false))

(event `Lumière`
  (bind _returnvalue (`GameplayStatics.GetActorOfClass` "/Game/G2S1_project/Blueprints/Bp_chat.Bp_chat_C"))
  (if (`self.IsOverlappingActor` _returnvalue)
    (bind _asbp_chat (cast `/Game/G2S1_project/Blueprints/Bp_chat` _returnvalue))
    (`/Game/G2S1_project/Blueprints/Bp_chat.control_Arthur` _asbp_chat)
    (set `self.allumé` true)
    (bind _outactors (`GameplayStatics.GetAllActorsOfClass` "/Game/G2S1_project/Blueprints/Bp_SalleSombre.Bp_SalleSombre_C"))
    (for _array_element _outactors
      (if (== (`/Game/G2S1_project/Blueprints/Bp_SalleSombre.Numéro Salle` _array_element) (`self.Numéro interrupteur`))
        (`SceneComponent.SetVisibility` (`/Game/G2S1_project/Blueprints/Bp_SalleSombre.Obscurité` _array_element) false false)
        (`PrimitiveComponent.SetCollisionEnabled` (`/Game/G2S1_project/Blueprints/Bp_SalleSombre.Collision` _array_element) "NoCollision")
        (`PrimitiveComponent.SetCollisionEnabled` (`/Game/G2S1_project/Blueprints/Bp_SalleSombre.CollisionEst` _array_element) "NoCollision")
        (`PrimitiveComponent.SetCollisionEnabled` (`/Game/G2S1_project/Blueprints/Bp_SalleSombre.CollisionSud` _array_element) "NoCollision")
        (`PrimitiveComponent.SetCollisionEnabled` (`/Game/G2S1_project/Blueprints/Bp_SalleSombre.CollisionNord` _array_element) "NoCollision")
        (`PrimitiveComponent.SetCollisionEnabled` (`/Game/G2S1_project/Blueprints/Bp_SalleSombre.CollisionOuest` _array_element) "NoCollision")))))

(event `self.ReceiveActorEndOverlap`
  (params (OtherActor :type "Actor Object Reference"))
  (bind _returnvalue (`GameplayStatics.GetActorOfClass` "/Game/G2S1_project/Blueprints/Bp_chat.Bp_chat_C"))
  (if (== _returnvalue OtherActor)
    (if (`self.allumé`)
      (set `self.allumé` false)
      (bind _outactors (`GameplayStatics.GetAllActorsOfClass` "/Game/G2S1_project/Blueprints/Bp_SalleSombre.Bp_SalleSombre_C"))
      (for _array_element _outactors
        (if (== (`/Game/G2S1_project/Blueprints/Bp_SalleSombre.Numéro Salle` _array_element) (`self.Numéro interrupteur`))
          (`SceneComponent.SetVisibility` (`/Game/G2S1_project/Blueprints/Bp_SalleSombre.Obscurité` _array_element) true false)
          (`PrimitiveComponent.SetCollisionEnabled` (`/Game/G2S1_project/Blueprints/Bp_SalleSombre.Collision` _array_element) "QueryAndPhysics")
          (`PrimitiveComponent.SetCollisionEnabled` (`/Game/G2S1_project/Blueprints/Bp_SalleSombre.CollisionEst` _array_element) "QueryAndPhysics")
          (`PrimitiveComponent.SetCollisionEnabled` (`/Game/G2S1_project/Blueprints/Bp_SalleSombre.CollisionSud` _array_element) "QueryAndPhysics")
          (`PrimitiveComponent.SetCollisionEnabled` (`/Game/G2S1_project/Blueprints/Bp_SalleSombre.CollisionNord` _array_element) "QueryAndPhysics")
          (`PrimitiveComponent.SetCollisionEnabled` (`/Game/G2S1_project/Blueprints/Bp_SalleSombre.CollisionOuest` _array_element) "QueryAndPhysics"))))))

(event `lacher interrupteur`
  (bind _returnvalue (`GameplayStatics.GetActorOfClass` "/Game/G2S1_project/Blueprints/Bp_chat.Bp_chat_C"))
  (if (`self.IsOverlappingActor` _returnvalue)
    (set `self.allumé` true)
    (bind _outactors (`GameplayStatics.GetAllActorsOfClass` "/Game/G2S1_project/Blueprints/Bp_SalleSombre.Bp_SalleSombre_C"))
    (for _array_element _outactors
      (if (== (`/Game/G2S1_project/Blueprints/Bp_SalleSombre.Numéro Salle` _array_element) (`self.Numéro interrupteur`))
        (`SceneComponent.SetVisibility` (`/Game/G2S1_project/Blueprints/Bp_SalleSombre.Obscurité` _array_element) true false)
        (`PrimitiveComponent.SetCollisionEnabled` (`/Game/G2S1_project/Blueprints/Bp_SalleSombre.Collision` _array_element) "QueryAndPhysics")
        (`PrimitiveComponent.SetCollisionEnabled` (`/Game/G2S1_project/Blueprints/Bp_SalleSombre.CollisionEst` _array_element) "QueryAndPhysics")
        (`PrimitiveComponent.SetCollisionEnabled` (`/Game/G2S1_project/Blueprints/Bp_SalleSombre.CollisionSud` _array_element) "QueryAndPhysics")
        (`PrimitiveComponent.SetCollisionEnabled` (`/Game/G2S1_project/Blueprints/Bp_SalleSombre.CollisionNord` _array_element) "QueryAndPhysics")
        (`PrimitiveComponent.SetCollisionEnabled` (`/Game/G2S1_project/Blueprints/Bp_SalleSombre.CollisionOuest` _array_element) "QueryAndPhysics")))))

(fn `UserConstructionScript`)