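; Audio manager Blueprint that handles music for the two worlds and footstep sounds for the characters Catty and Arthur.
; BeginPlay creates all four audio components, and a separate Ambiance event adds a quieter one.
; The changementmonde event uses a FlipFlop to swap volumes between MondeReel and OtherWorld, keeping the inactive track near-silent.
; Tick looks up Bp_chat and Bp_gorille each frame, raising or nearly muting their footstep loops based on velocity.
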(event `Ambiance`
  (bind _returnvalue (`AddComponent|NODE_AddAudioComponent-0`))
  (`AudioComponent.SetVolumeMultiplier` _returnvalue 0.4))

(event `self.ReceiveBeginPlay`
  (bind _returnvalue (`AddComponent|NODE_AddAudioComponent-2`))
  (bind _output_get (set `self.MondeReel` _returnvalue))
  (`AudioComponent.SetVolumeMultiplier` _output_get 1.0)
  (bind _returnvalue_2 (`AddComponent|NODE_AddAudioComponent-3`))
  (bind _output_get_2 (set `self.OtherWorld` _returnvalue_2))
  (`AudioComponent.SetVolumeMultiplier` _output_get_2 0.01)
  (bind _returnvalue_3 (`AddComponent|NODE_AddAudioComponent-4`))
  (bind _output_get_3 (set `self.PasCatty` _returnvalue_3))
  (`AudioComponent.SetVolumeMultiplier` _output_get_3 3.0)
  (bind _returnvalue_4 (`AddComponent|NODE_AddAudioComponent-5`))
  (bind _output_get_4 (set `self.PasArthur` _returnvalue_4))
  (`AudioComponent.SetVolumeMultiplier` _output_get_4 3.0))

(event `changement monde`
  ;[1 1 1] changement monde musique
  (`/Engine/EditorBlueprintResources/StandardMacros.FlipFlop`
    (:`A`
      (bind _asaudio_component (cast `AudioComponent` (`self.MondeReel`)))
      (`AudioComponent.SetVolumeMultiplier` _asaudio_component 0.01)
      (bind _asaudio_component_2 (cast `AudioComponent` (`self.OtherWorld`)))
      (`AudioComponent.SetVolumeMultiplier` _asaudio_component_2 1.0))
    (:`B`
      (bind _asaudio_component_3 (cast `AudioComponent` (`self.MondeReel`)))
      (`AudioComponent.SetVolumeMultiplier` _asaudio_component_3 1.0)
      (bind _asaudio_component_4 (cast `AudioComponent` (`self.OtherWorld`)))
      (`AudioComponent.SetVolumeMultiplier` _asaudio_component_4 0.01))))

(event `self.ReceiveTick`
  (params (DeltaSeconds :type "Float (single-precision)"))
  ;[1 1 1] bruits de pas catty
  (bind _returnvalue (`GameplayStatics.GetActorOfClass` "/Game/G2S1_project/Blueprints/Bp_chat.Bp_chat_C"))
  (if (== (`self.GetVelocity` _returnvalue) (0.0 0.0 0.0) :`ErrorTolerance` 0.1)
    (set `self.CattyMarche` false)
    (`AudioComponent.SetVolumeMultiplier` (`self.PasCatty`) 0.01)
    (else
      (set `self.CattyMarche` true)
      (`AudioComponent.SetVolumeMultiplier` (`self.PasCatty`) 3.0)))
  ;[1 1 1] bruits de pas Arthur
  (bind _returnvalue_2 (`GameplayStatics.GetActorOfClass` "/Game/G2S1_project/Blueprints/Bp_gorille.Bp_gorille_C"))
  (if (== (`self.GetVelocity` _returnvalue_2) (0.0 0.0 0.0) :`ErrorTolerance` 0.1)
    (`AudioComponent.SetVolumeMultiplier` (`self.PasArthur`) 0.01)
    (else
      (`AudioComponent.SetVolumeMultiplier` (`self.PasArthur`) 3.0))))

(fn `UserConstructionScript`)