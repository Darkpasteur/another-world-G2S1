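; Obscuru is a pawn that starts moving forward on its own after the first actor overlaps it.
; That overlap finds the Musiques actor, calls its Ambiance event and latches the Collidé flag so the trigger does not repeat.
; While the flag is set, Tick feeds half-strength movement input along the forward direction of the control rotation's yaw.
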(event `self.ReceiveTick`
  (params (DeltaSeconds :type "Float (single-precision)"))
  (bind (_returnvalue_roll _returnvalue_pitch _returnvalue_yaw) (`KismetMathLibrary.BreakRotator` (`self.GetControlRotation`)))
  (if (`self.collidé`)
    (`self.AddMovementInput` (`KismetMathLibrary.GetForwardVector` (`KismetMathLibrary.MakeRotator` 0.0 0.0 _returnvalue_yaw)) 0.5)))

(event `self.ReceiveActorBeginOverlap`
  (params (OtherActor :type "Actor Object Reference"))
  (if (not (`self.collidé`))
    (bind _returnvalue (`GameplayStatics.GetActorOfClass` "/Game/G2S1_project/Blueprints/Musiques.Musiques_C"))
    (bind _asmusiques (cast `/Game/G2S1_project/Blueprints/Musiques` _returnvalue))
    (`/Game/G2S1_project/Blueprints/Musiques.Ambiance` _asmusiques)
    (set `self.collidé` true)))

(fn `UserConstructionScript`)