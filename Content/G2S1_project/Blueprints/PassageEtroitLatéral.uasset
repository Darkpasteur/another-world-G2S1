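; Narrow lateral passage actor that lets the cat character (Bp_chat) cross from one side to the other.
; On overlap, it filters by the hardcoded instance name Bp_chat_C_1, then checks the right or left collision to choose the crossing direction.
; It briefly disables its three collision components, calls the cat's matching passage function, and restores collision after a short delay.
; Any other overlapping actor only prints a failure message.
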(event `self.ReceiveActorBeginOverlap`
  (params (OtherActor :type "Actor Object Reference"))
  (if (`KismetStringLibrary.NotEqual_StrStr` (`KismetStringLibrary.Conv_ObjectToString` OtherActor) "Bp_chat_C_1")
    (`KismetSystemLibrary.PrintString` "Passage étroit RATE")
    (elif (`PrimitiveComponent.IsOverlappingActor` (`self.CollisionDroite`) OtherActor)
      (`PrimitiveComponent.SetCollisionEnabled` (`self.Cubecollide`) "NoCollision")
      (`PrimitiveComponent.SetCollisionEnabled` (`self.CollisionGauche`) "NoCollision")
      (`PrimitiveComponent.SetCollisionEnabled` (`self.CollisionDroite`) "NoCollision")
      (bind _asbp_chat (cast `/Game/G2S1_project/Blueprints/Bp_chat` OtherActor))
      (`/Game/G2S1_project/Blueprints/Bp_chat.PassageDroiteGauche` _asbp_chat)
      (`KismetSystemLibrary.Delay` 0.2)
      (`PrimitiveComponent.SetCollisionEnabled` (`self.Cubecollide`) "QueryAndPhysics")
      (`PrimitiveComponent.SetCollisionEnabled` (`self.CollisionGauche`) "QueryAndPhysics")
      (`PrimitiveComponent.SetCollisionEnabled` (`self.CollisionDroite`) "QueryAndPhysics")
      (elif (`PrimitiveComponent.IsOverlappingActor` (`self.CollisionGauche`) OtherActor)
        (`PrimitiveComponent.SetCollisionEnabled` (`self.Cubecollide`) "NoCollision")
        (`PrimitiveComponent.SetCollisionEnabled` (`self.CollisionGauche`) "NoCollision")
        (`PrimitiveComponent.SetCollisionEnabled` (`self.CollisionDroite`) "NoCollision")
        (bind _asbp_chat_2 (cast `/Game/G2S1_project/Blueprints/Bp_chat` OtherActor))
        (`/Game/G2S1_project/Blueprints/Bp_chat.PassageGaucheDroite` _asbp_chat_2)
        (`KismetSystemLibrary.Delay` 0.2)
        (`PrimitiveComponent.SetCollisionEnabled` (`self.Cubecollide`) "QueryAndPhysics")
        (`PrimitiveComponent.SetCollisionEnabled` (`self.CollisionGauche`) "QueryAndPhysics")
        (`PrimitiveComponent.SetCollisionEnabled` (`self.CollisionDroite`) "QueryAndPhysics")))))

(fn `UserConstructionScript`)