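; Pressure plate actor that opens numbered doors when the gorilla (Bp_gorille) or a Caisse2 crate overlaps it.
; On overlap it hides and disables collision on PlaqueCylindre, then opens every Bp_Porte and Bp_PorteS whose number matches NuméroPlaque.
; End overlap restores the cylinder for any actor, as its branch is hardwired true, and sends nothing to the doors.
; Debug prints remain in the door loop.
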(event `self.ReceiveActorBeginOverlap`
  (params (OtherActor :type "Actor Object Reference"))
  (bind _returnvalue (`GameplayStatics.GetActorOfClass` "/Game/G2S1_project/Blueprints/Bp_gorille.Bp_gorille_C"))
  (if (== _returnvalue OtherActor)
    (`SceneComponent.SetVisibility` (`self.plaque cylindre`) false false :!label _label)
    (`PrimitiveComponent.SetCollisionEnabled` (`self.plaque cylindre`) "NoCollision")
    (bind _outactors (`GameplayStatics.GetAllActorsOfClass` "/Game/G2S1_project/Blueprints/Portes/Bp_Porte.Bp_Porte_C"))
    (for _array_element _outactors
      (bind `_numéroporte` (`/Game/G2S1_project/Blueprints/Portes/Bp_Porte.numéroporte` _array_element))
      (`KismetSystemLibrary.PrintString` (`KismetStringLibrary.Conv_IntToString` `_numéroporte`))
      (if (== `_numéroporte` (`self.Numéro plaque`))
        (`KismetSystemLibrary.PrintString` "Hello")
        (bind _output_get (set `self.Array Element` _array_element))
        (bind _asbp_porte (cast `/Game/G2S1_project/Blueprints/Portes/Bp_Porte` _output_get)
          (:`then`
            (`/Game/G2S1_project/Blueprints/Portes/Bp_Porte.OuvrirPorte` _asbp_porte))
          (:`CastFailed`
            (`KismetSystemLibrary.PrintString` "cast raté")))))
    (bind _outactors_2 (`GameplayStatics.GetAllActorsOfClass` "/Game/G2S1_project/Blueprints/Portes/Bp_PorteS.Bp_PorteS_C"))
    (for _array_element_2 _outactors_2
      (if (== (`/Game/G2S1_project/Blueprints/Portes/Bp_PorteS.numéroporteS` _array_element_2) (`self.Numéro plaque`))
        (bind _output_get_2 (set `self.Array Element_0` _array_element_2))
        (bind _asbp_porte_s (cast `/Game/G2S1_project/Blueprints/Portes/Bp_PorteS` _output_get_2))
        (`/Game/G2S1_project/Blueprints/Portes/Bp_PorteS.PorteOuvre` _asbp_porte_s)))
    (else
      (bind _outactors_3 (`GameplayStatics.GetAllActorsOfClass` "/Game/G2S1_project/Blueprints/caisse2.caisse2_C"))
      (for _array_element_3 _outactors_3
        (if (== _array_element_3 OtherActor)
          (goto _label))))))

(event `self.ReceiveActorEndOverlap`
  (params (OtherActor :type "Actor Object Reference"))
  (bind _returnvalue (`GameplayStatics.GetActorOfClass` "/Game/G2S1_project/Blueprints/Bp_gorille.Bp_gorille_C"))
  (if true
    (`SceneComponent.SetVisibility` (`self.plaque cylindre`) true false :!label _label_2)
    (`PrimitiveComponent.SetCollisionEnabled` (`self.plaque cylindre`) "QueryAndPhysics")
    (else
      (bind _outactors (`GameplayStatics.GetAllActorsOfClass` "/Game/G2S1_project/Blueprints/caisse2.caisse2_C"))
      (for _array_element _outactors
        (if (== _array_element OtherActor)
          (goto _label_2))))))

(fn `UserConstructionScript`)