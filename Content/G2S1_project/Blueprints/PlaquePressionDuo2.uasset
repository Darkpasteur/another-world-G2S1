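; Second half of a two-plate pressure puzzle that opens doors when the gorilla or a Caisse2 crate steps on it.
; On overlap it hides the plate cylinder, disables its collision, and finds Bp_Porte and Bp_PorteS doors sharing its plate number.
; Those doors open only if the matching PlaquePressionDuo1 is already activated.
; Any actor ending overlap restores the cylinder, as that branch is hardwired true; doors are never closed here.
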(event `self.ReceiveActorBeginOverlap`
  (params (OtherActor :type "Actor Object Reference"))
  (bind _returnvalue (`GameplayStatics.GetActorOfClass` "/Game/G2S1_project/Blueprints/Bp_gorille.Bp_gorille_C"))
  (if (== _returnvalue OtherActor)
    (`SceneComponent.SetVisibility` (`self.plaque cylindre`) false false :!label _label)
    (`PrimitiveComponent.SetCollisionEnabled` (`self.plaque cylindre`) "NoCollision")
    (bind _outactors (`GameplayStatics.GetAllActorsOfClass` "/Game/G2S1_project/Blueprints/Portes/Bp_Porte.Bp_Porte_C"))
    (for _array_element _outactors
      (if (== (`/Game/G2S1_project/Blueprints/Portes/Bp_Porte.numéroporte` _array_element) (`self.Numéro plaque`))
        (set `self.porte` _array_element)
        (bind _outactors_2 (`GameplayStatics.GetAllActorsOfClass` "/Game/G2S1_project/Blueprints/PlaquePressionDuo1.PlaquePressionDuo1_C"))
        (for _array_element_2 _outactors_2
          (if (== (`/Game/G2S1_project/Blueprints/PlaquePressionDuo1.Numéro plaque` _array_element_2) (`self.Numéro plaque`))
            (if (`/Game/G2S1_project/Blueprints/PlaquePressionDuo1.Activée` _array_element_2)
              (bind _asbp_porte (cast `/Game/G2S1_project/Blueprints/Portes/Bp_Porte` (`self.porte`)))
              (`/Game/G2S1_project/Blueprints/Portes/Bp_Porte.OuvrirPorte` _asbp_porte))))))
    (bind _outactors_3 (`GameplayStatics.GetAllActorsOfClass` "/Game/G2S1_project/Blueprints/Portes/Bp_PorteS.Bp_PorteS_C"))
    (for _array_element_3 _outactors_3
      (if (== (`/Game/G2S1_project/Blueprints/Portes/Bp_PorteS.numéroporteS` _array_element_3) (`self.Numéro plaque`))
        (set `self.porteS` _array_element_3)
        (bind _outactors_4 (`GameplayStatics.GetAllActorsOfClass` "/Game/G2S1_project/Blueprints/PlaquePressionDuo1.PlaquePressionDuo1_C"))
        (for _array_element_4 _outactors_4
          (if (== (`/Game/G2S1_project/Blueprints/PlaquePressionDuo1.Numéro plaque` _array_element_4) (`self.Numéro plaque`))
            (if (`/Game/G2S1_project/Blueprints/PlaquePressionDuo1.Activée` _array_element_4)
              (bind _asbp_porte_s (cast `/Game/G2S1_project/Blueprints/Portes/Bp_PorteS` (`self.porteS`)))
              (`/Game/G2S1_project/Blueprints/Portes/Bp_PorteS.PorteOuvre` _asbp_porte_s))))))
    (else
      (bind _returnvalue_2 (`GameplayStatics.GetActorOfClass` "/Game/G2S1_project/Blueprints/caisse2.caisse2_C"))
      (if (== _returnvalue_2 OtherActor)
        (goto _label)))))

(event `self.ReceiveActorEndOverlap`
  (params (OtherActor :type "Actor Object Reference"))
  (bind _returnvalue (`GameplayStatics.GetActorOfClass` "/Game/G2S1_project/Blueprints/Bp_gorille.Bp_gorille_C"))
  (if true
    (`SceneComponent.SetVisibility` (`self.plaque cylindre`) true false :!label _label_2)
    (`PrimitiveComponent.SetCollisionEnabled` (`self.plaque cylindre`) "QueryAndPhysics")
    (else
      (bind _returnvalue_2 (`GameplayStatics.GetActorOfClass` "/Game/G2S1_project/Blueprints/caisse2.caisse2_C"))
      (if (== _returnvalue_2 OtherActor)
        (goto _label_2)))))

(fn `UserConstructionScript`)