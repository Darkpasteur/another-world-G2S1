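; Bp_PorteE is a door that shows a widget prompt while the cat or gorilla character stands in its collision volume and the door is still closed.
; The OuvrirPorte event plays a timeline that swings the PivotD component up to -90 degrees in world yaw and marks the door as open.
; Leaving the volume hides the widget, and the file contains no closing logic.
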(event `self.PorteCollision.OnComponentEndOverlap`
  (params (OverlappedComponent :type "PrimitiveComponent Object Reference") (OtherActor :type "Actor Object Reference") (OtherComp :type "PrimitiveComponent Object Reference") (OtherBodyIndex :type Integer))
  (`SceneComponent.SetVisibility` (`self.Widget`) false false))

(event `self.PorteCollision.OnComponentBeginOverlap`
  (params (OverlappedComponent :type "PrimitiveComponent Object Reference") (OtherActor :type "Actor Object Reference") (OtherComp :type "PrimitiveComponent Object Reference") (OtherBodyIndex :type Integer) (bFromSweep :type Boolean) (SweepResult :type "HitResult Structure (by ref)"))
  (cast `/Game/G2S1_project/Blueprints/Bp_chat` OtherActor
    (:`then`
      _)
    (:`CastFailed`
      (cast `/Game/G2S1_project/Blueprints/Bp_gorille` OtherActor)))
  (if (not (`self.Ouverte`))
    (`SceneComponent.SetVisibility` (`self.Widget`) true false)))

(event `OuvrirPorte`
  (bind (_direction _portetimer) (`Timeline|TLPorte`)
    (:`Update`
      (`SceneComponent.K2_SetWorldRotation` (`self.PivotD`) (`KismetMathLibrary.MakeRotator` 0.0 0.0 (* _portetimer -90.0)) false false)
      (set `self.Ouverte` true))))

(fn `UserConstructionScript`)