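; Key pickup actor that plays a short dialogue between Cathie and Arthur, then unlocks the key door.
; Overlap by Bp_chat deactivates that character's movement and shows the WBP_DialogueCle widget once.
; Each ParlerCle event advances an index into line and portrait arrays to update the widget.
; At the end index it restores movement, removes the widget, sets Cle on Bp_PorteCle and destroys itself.
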(event `self.ReceiveActorBeginOverlap`
  (params (OtherActor :type "Actor Object Reference"))
  (bind _returnvalue (`GameplayStatics.GetActorOfClass` (`GameplayStatics.GetObjectClass` OtherActor)))
  (bind _asbp_chat (cast `/Game/G2S1_project/Blueprints/Bp_chat` _returnvalue))
  (`ActorComponent.Deactivate` (`Character.CharacterMovement` _asbp_chat))
  (`/Engine/EditorBlueprintResources/StandardMacros.DoOnce` false
    (:`Completed`
      (bind _returnvalue_2 (`|CreateWidget` "/Game/G2S1_project/Ui/WBP_DialogueCle.WBP_DialogueCle_C"))
      (bind _output_get (set `self.dialCle` _returnvalue_2))
      (`UserWidget.AddToViewport` _output_get 0))))

(event `ParlerCle`
  (bind _asbp_chat (cast `/Game/G2S1_project/Blueprints/Bp_chat` (stale `self.ReceiveActorBeginOverlap` _returnvalue)))
  (bind _result (`/Engine/EditorBlueprintResources/StandardMacros.IncrementInt` (`self.Parler_Index`))
    (:`  `
      (`TextBlock.SetText` (`/Game/G2S1_project/Ui/WBP_DialogueCle.CathieText` (`self.dialCle`)) (`KismetTextLibrary.Conv_StringToText` (`|GetArrayItem` (`self.Dialogues Cathie`) (`self.Parler_Index`))))
      (`TextBlock.SetText` (`/Game/G2S1_project/Ui/WBP_DialogueCle.Arthurtext` (`self.dialCle`)) (`KismetTextLibrary.Conv_StringToText` (`|GetArrayItem` (`self.DialoguesArthur`) (`self.Parler_Index`))))
      (`Image.SetBrush` (`/Game/G2S1_project/Ui/WBP_DialogueCle.PortraitCathie` (`self.dialCle`)) (make `SlateBrush` (32.0 32.0) (struct) (struct :`SpecifiedColor` (struct :`R` 1.0 :`G` 1.0 :`B` 1.0 :`A` 1.0) :`ColorUseRule` "UseColor_Specified") (struct :`CornerRadii` (struct :`W` 1.0) :`Color` (struct :`SpecifiedColor` (struct) :`ColorUseRule` "UseColor_Specified") :`RoundingType` "HalfHeightRadius") (`|GetArrayItem` (`self.Portraits`) (`self.Parler_Index`))))
      (`Image.SetBrush` (`/Game/G2S1_project/Ui/WBP_DialogueCle.PortraitArthur` (`self.dialCle`)) (make `SlateBrush` (32.0 32.0) (struct) (struct :`SpecifiedColor` (struct :`R` 1.0 :`G` 1.0 :`B` 1.0 :`A` 1.0) :`ColorUseRule` "UseColor_Specified") (struct :`CornerRadii` (struct :`W` 1.0) :`Color` (struct :`SpecifiedColor` (struct) :`ColorUseRule` "UseColor_Specified") :`RoundingType` "HalfHeightRadius") (`|GetArrayItem` (`self.PortraitsArthur`) (`self.Parler_Index`))))
      (if (== _result 1)
        (`ActorComponent.Activate` (`Character.CharacterMovement` _asbp_chat) false)
        (`Widget.RemoveFromParent` (`self.dialCle`))
        (bind _returnvalue (`GameplayStatics.GetActorOfClass` "/Game/G2S1_project/Blueprints/Portes/Bp_PorteCle.Bp_PorteCle_C"))
        (set `/Game/G2S1_project/Blueprints/Portes/Bp_PorteCle.Cle` true _returnvalue)
        (`self.K2_DestroyActor`)))))

(fn `UserConstructionScript`)